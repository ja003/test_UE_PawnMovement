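; BP_MyPawn is an AI pawn that navigates to a point offset from its spawn location by its Target vector.
; BeginPlay issues a simple move to that point through the pawn's controller and draws a temporary debug sphere there.
; A RandomWander event moves to a random reachable nearby point and prints a location, but the looping timer meant to trigger it is disconnected.
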(event Custom|RandomWander
  (bind _returnvalue (Transformation|GetActorLocation))
  (bind _randomlocation (AI|Navigation|GetRandomReachablePointinRadius _returnvalue 5e+02 0 0))
  (AI|Navigation|SimpleMovetoLocation (Pawn|GetController) _randomlocation)
  (Development|PrintString (Utilities|String|ToString(Vector) _randomlocation)))

(event EventBeginPlay
  (bind _returnvalue (Transformation|GetActorLocation))
  (bind _target (Variables|Default|GetTarget))
  (bind _returnvalue_2 (+ _target _returnvalue))
  (AI|Navigation|SimpleMovetoLocation (Pawn|GetController) _returnvalue_2)
  (Rendering|Debug|DrawDebugSphere _returnvalue_2 1e+02 12 "(R=1.000000,G=1.000000,B=1.000000,A=1.000000)" 5.0))

(fn ConstructionScript)