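; AI character Blueprint that moves itself with simple navigation move requests.
; On BeginPlay it makes a single move to its Target offset added to its current location.
; A RandomWander event moves to a random reachable nearby point and prints a separately re-rolled point, but its looping timer is disconnected and never runs.
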(event Custom|RandomWander
  (bind _returnvalue (Transformation|GetActorLocation))
  (bind _randomlocation (AI|Navigation|GetRandomReachablePointinRadius _returnvalue 5e+02 0 0))
  (AI|Navigation|SimpleMovetoLocation (Pawn|GetController) _randomlocation)
  (Development|PrintString (Utilities|String|ToString(Vector) _randomlocation)))

(event EventBeginPlay
  (AI|Navigation|SimpleMovetoLocation (Pawn|GetController) (+ (Variables|Default|GetTarget) (Transformation|GetActorLocation))))

(fn ConstructionScript)